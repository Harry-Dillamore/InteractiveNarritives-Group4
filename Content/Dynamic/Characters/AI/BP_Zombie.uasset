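; Zombie AI character that trades melee hits with the first-person player.
; Hit plays a sound and impact montage, holding BeingHit for the montage's duration behind a DoOnce; both LeftHand branches use the same montage.
; While IsPunching is set, PunchTrace re-calls itself after short delays, capsule-tracing at the right hand until it finds the player, then calls the player's Hit and shakes the camera.
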(event Custom|Hit
  (Utilities|FlowControl|DoOnce false :!label _label
    (:Completed
      (Audio|PlaySoundatLocation 0 (Transformation|GetActorLocation) "0, 0, 0" 1.0 1.0 0.0 0 0 0 0)
      (Variables|Default|SetBeingHit true)
      (bind _returnvalue (Animation|PlayAnimMontage (select (Variables|/Game/Dynamic/Blueprints/Core/MC/BP_FirstPersonCharacter.BP_FirstPersonCharacter_C|GetLeftHand (Variables|Default|GetChar%20REF)) "/Game/Static/Fighting_Animations/Animations/Impact_mixamo_com_Montage.Impact_mixamo_com_Montage" "/Game/Static/Fighting_Animations/Animations/Impact_mixamo_com_Montage.Impact_mixamo_com_Montage") 1.0 "None"))
      (Utilities|FlowControl|Delay _returnvalue)
      (Variables|Default|SetBeingHit false)
      (goto _label Reset))))

(event Custom|Punch%20Trace
  (bind _mesh (Variables|Character|GetMesh))
  (bind _returnvalue (Transformation|GetSocketLocation _mesh "hand_r"))
  (if (Variables|Default|GetIsPunching)
    (bind (_outhit _returnvalue_2) (Class|KismetSystemLibrary|CapsuleTraceSingleforObjects _returnvalue _returnvalue 11.0 11.0 (Utilities|Array|MakeArray "ObjectTypeQuery3") false 0 "None" true))
    (if _returnvalue_2
      (bind _asbp_first_person_character (Utilities|Casting|CastToBP_FirstPersonCharacter (.HitActor (Collision|BreakHitResult _outhit)))
        (:then
          (Default|Hit _asbp_first_person_character)
          (Camera|PlayWorldCameraShake "/Game/Dynamic/Blueprints/Core/MC/BP_CameraShake.BP_CameraShake_C" _returnvalue 0.0 1e+02))
        (:CastFailed
          (Utilities|FlowControl|Delay 0.01 :!label _label)
          (CallFunction|PunchTrace)))
      (else
        (goto _label)))))

(event EventBeginPlay
  (bind _asbp_first_person_character (Utilities|Casting|CastToBP_FirstPersonCharacter (Game|GetPlayerCharacter 0)))
  (Variables|Default|SetChar%20REF _asbp_first_person_character))

(event Collision|EventActorBeginOverlap
  (params (OtherActor :type Actor%20Object%20Reference)))

(event EventTick
  (params (DeltaSeconds :type Float%20%28single-precision%29)))

(fn ConstructionScript)