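; BP_NPC_BasementDweller is an interactable NPC that talks to the player through its dialogue component.
; Interact starts dialogue at a stored starting ID.
; Named dialogue events change that ID so later conversations reflect how the last one went.
; The gas events also add a full or half-full gas can gameplay tag to the cached first-person player's owned tags.
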(event EventInteract
  (Default|StartDialog (Variables|Default|GetBPC_DialogueComponent) (Variables|Default|GetStarting%20Dialog%20ID_0)))

(event EventBeginPlay
  (bind _asbp_first_person_character (Utilities|Casting|CastToBP_FirstPersonCharacter (Game|GetPlayerCharacter 0)))
  (Variables|Default|SetPlayerRef _asbp_first_person_character))

(event EventDialogueEvent
  (params (DialogEventName :type Text))
  (bind _playerref (Variables|Default|GetPlayerRef))
  (bind _ownedgameplaytags (Variables|/Game/Dynamic/Blueprints/Core/MC/BP_FirstPersonCharacter.BP_FirstPersonCharacter_C|GetOwnedGameplayTags _playerref))
  (switch string (Utilities|String|ToString(Text) DialogEventName)
    (:Asshole
      (Variables|Default|SetStarting%20Dialog%20ID_0 75))
    (:Rude
      (Variables|Default|SetStarting%20Dialog%20ID_0 76))
    (:SpokenTo
      (Variables|Default|SetStarting%20Dialog%20ID_0 64))
    (:EndDialogue
      (Variables|Default|SetStarting%20Dialog%20ID_0 87))
    (:GiveGas
      (Variables|Default|SetStarting%20Dialog%20ID_0 87)
      (GameplayTags|AddGameplayTag _ownedgameplaytags "(TagName=\"Dialog.HasItem.GasCan(Full)\")" :!class /Script/GameplayTags.BlueprintGameplayTagLibrary))
    (:GivehalfGas
      (Variables|Default|SetStarting%20Dialog%20ID_0 87)
      (GameplayTags|AddGameplayTag _ownedgameplaytags "(TagName=\"Dialog.HasItem.GasCan(HalfFull)\")" :!class /Script/GameplayTags.BlueprintGameplayTagLibrary))))

(fn ConstructionScript
  (|CallParentFunction))