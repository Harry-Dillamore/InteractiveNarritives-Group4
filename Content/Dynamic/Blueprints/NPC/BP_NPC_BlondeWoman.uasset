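; BP_NPC_BlondeWoman is the Blueprint for the blonde woman NPC, who starts a dialogue when the player interacts with her.
; It caches the first-person player character on BeginPlay and passes the current starting dialog ID to its dialogue component.
; A "Spoken to" dialogue event switches that starting ID for later conversations and adds a gameplay tag to the player recording that she has been spoken to.
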(event EventInteract
  (Default|StartDialog (Variables|Default|GetBPC_DialogueComponent) (Variables|Default|GetStarting%20Dialog%20ID_0)))

(event EventBeginPlay
  (bind _asbp_first_person_character (Utilities|Casting|CastToBP_FirstPersonCharacter (Game|GetPlayerCharacter 0)))
  (Variables|Default|SetPlayerRef _asbp_first_person_character))

(event EventDialogueEvent
  (params (DialogEventName :type Text))
  (switch string (Utilities|String|ToString(Text) DialogEventName)
    (:SpokenTo
      (Variables|Default|SetStarting%20Dialog%20ID_0 18)
      (GameplayTags|AddGameplayTag (Variables|/Game/Dynamic/Blueprints/Core/MC/BP_FirstPersonCharacter.BP_FirstPersonCharacter_C|GetOwnedGameplayTags (Variables|Default|GetPlayerRef)) "(TagName=\"Dialog.HasSpoken.BlondeWoman\")" :!class /Script/GameplayTags.BlueprintGameplayTagLibrary))))

(fn ConstructionScript
  (|CallParentFunction))