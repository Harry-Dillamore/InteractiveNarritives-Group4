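; BP_NPC_OldMan2 is an old man NPC that the player talks to through a dialogue component.
; Interact starts dialogue at a stored starting ID, and BeginPlay caches the first-person character.
; Named dialogue events add gameplay tags to the player for having spoken, getting the gun and being nice.
; The spoken-to and end-dialogue events also change the starting ID for later conversations.
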(event EventDialogueEvent
  (params (DialogEventName :type Text))
  (bind _playerref (Variables|Default|GetPlayerRef))
  (bind _ownedgameplaytags (Variables|/Game/Dynamic/Blueprints/Core/MC/BP_FirstPersonCharacter.BP_FirstPersonCharacter_C|GetOwnedGameplayTags _playerref))
  (switch string (Utilities|String|ToString(Text) DialogEventName)
    (:SpokenTo
      (Variables|Default|SetStarting%20Dialog%20ID_0 55)
      (GameplayTags|AddGameplayTag _ownedgameplaytags "(TagName=\"Dialog.HasSpoken.OldMan\")" :!class /Script/GameplayTags.BlueprintGameplayTagLibrary))
    (:GetGun
      (GameplayTags|AddGameplayTag _ownedgameplaytags "(TagName=\"Dialog.HasItem.Gun\")" :!class /Script/GameplayTags.BlueprintGameplayTagLibrary))
    (:WasNice
      (GameplayTags|AddGameplayTag _ownedgameplaytags "(TagName=\"Dialog.OldMan.Nice\")" :!class /Script/GameplayTags.BlueprintGameplayTagLibrary))
    (:EndDialogue
      (Variables|Default|SetStarting%20Dialog%20ID_0 58))))

(event EventInteract
  (Default|StartDialog (Variables|Default|GetBPC_DialogueComponent) (Variables|Default|GetStarting%20Dialog%20ID_0)))

(event EventBeginPlay
  (bind _asbp_first_person_character (Utilities|Casting|CastToBP_FirstPersonCharacter (Game|GetPlayerCharacter 0)))
  (Variables|Default|SetPlayerRef _asbp_first_person_character))

(fn ConstructionScript
  (|CallParentFunction))